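; Interactable affordance that works as a light switch, hiding or showing every ceiling light actor in the world.
; Its Interact override calls the parent, plays a switch sound, flips CurrentlyVisible and passes it as the hidden-in-game state of all CeilingLight_Blueprint actors.
; Despite its name, a true CurrentlyVisible hides the lights, and targets come from a class search, leaving ActorsToToggle unused.
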(fn `Interact`
  (bind _currentlyvisible (`self.CurrentlyVisible`))
  (`parent.Interact`)
  (`GameplayStatics.PlaySound2D` "/Game/Audio/light_switch.light_switch" 1.0 1.0 0.0 null null)
  (set `self.CurrentlyVisible` (not _currentlyvisible))
  (bind _outactors (`GameplayStatics.GetAllActorsOfClass` "/Game/Blueprints/CeilingLight_Blueprint.CeilingLight_Blueprint_C"))
  (for _array_element _outactors
    (`Actor.SetActorHiddenInGame` _array_element _currentlyvisible)))